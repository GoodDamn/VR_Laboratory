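; BP_shelf is a shelf actor that motion controllers can pick up and drop, with tracking for up to two grips at once.
; Pickup binds the static mesh to the hand through the passed-in physics constraint and stores it in the first or second slot.
; Drop breaks the matching stored constraint and promotes the second grip to the first slot when the first is released.
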(event `/Game/VirtualRealityBP/Blueprints/PickupActorInterface.Pickup`
  (params (Constraint :type "PhysicsConstraintComponent Object Reference") (Hand :type "StaticMeshComponent Object Reference"))
  (`PhysicsConstraintComponent.SetConstrainedComponents` Constraint Hand "None" (`self.StaticMeshComponent`) "None")
  (`self.Constraint`
    (:`then`
      (set `self.Constraint2` Constraint))
    (:`else`
      (set `self.Constraint` Constraint))))

(event `/Game/VirtualRealityBP/Blueprints/PickupActorInterface.Drop`
  (params (Constraint :type "PhysicsConstraintComponent Object Reference"))
  (bind _constraint (`self.Constraint`)
    (:`then`
      (if (== _constraint Constraint)
        (`PhysicsConstraintComponent.BreakConstraint` (`self.Constraint`))
        (set `self.Constraint` null)
        (bind _constraint2 (`self.Constraint2`)
          (:`then`
            (set `self.Constraint` _constraint2)
            (set `self.Constraint2` null))
          (:`else`))
        (else
          (bind _constraint2_2 (`self.Constraint2`)
            (:`then`
              (if (== _constraint2_2 Constraint)
                (`PhysicsConstraintComponent.BreakConstraint` (`self.Constraint2`))
                (set `self.Constraint2` null)))
            (:`else`)))))
    (:`else`)))

(fn `UserConstructionScript`)