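; BP_Washbasin is an interactive washbasin that a VR motion controller switches on and off by touch.
; Each overlap of a BP_MotionController with the Water component flips IsOpened, playing the audio from the start or stopping it.
; Audio is stopped on BeginPlay, and the toggle changes only the sound and the flag, with no visual change in the graph.
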(event `self.ReceiveBeginPlay`
  (`AudioComponent.Stop` (`self.Audio`)))

(event `self.Water.OnComponentBeginOverlap`
  (params (OverlappedComponent :type "PrimitiveComponent Object Reference") (OtherActor :type "Actor Object Reference") (OtherComp :type "PrimitiveComponent Object Reference") (OtherBodyIndex :type Integer) (bFromSweep :type Boolean) (SweepResult :type "HitResult Structure (by ref)"))
  (bind _audio (`self.Audio`))
  (cast `/Game/VirtualRealityBP/Blueprints/BP_MotionController` OtherActor)
  (if (`self.isOpened`)
    (`AudioComponent.Stop` _audio)
    (else
      (`AudioComponent.Play` _audio 0.0)))
  (set `self.isOpened` (not (`self.isOpened`))))

(fn `UserConstructionScript`)