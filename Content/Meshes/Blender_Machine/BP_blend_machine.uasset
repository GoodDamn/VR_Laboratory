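; Chemistry blending machine for VR that turns two placed substances into product flasks.
; Two trigger slots identify metals and flasks by class cast, store them as strings and change an indicator material.
; Tick calls Result once both slots fill, matching order-independent pairs to spawn products, often with hydrogen, or a dangerous flask for the secret pair and unknown mixes.
; Other overlaps toggle two lights and fade background audio near motion controllers.
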(event `self.ReceiveTick`
  (params (DeltaSeconds :type "Float (single-precision)"))
  (if (and (`self.DidSubstanceFill2`) (`self.DidSubstanceFill`))
    (`self.Result`)))

(event `self.ReceiveBeginPlay`
  (`AudioComponent.FadeOut` (`self.Audio`) 0.0 0.0 "Linear"))

(event `self.OFFer_general.OnComponentBeginOverlap`
  (params (OverlappedComponent :type "PrimitiveComponent Object Reference") (OtherActor :type "Actor Object Reference") (OtherComp :type "PrimitiveComponent Object Reference") (OtherBodyIndex :type Integer) (bFromSweep :type Boolean) (SweepResult :type "HitResult Structure (by ref)"))
  (bind _generallight (`self.GeneralLight`))
  (`SceneComponent.SetVisibility` _generallight (not (`SceneComponent.bVisible` _generallight)) false)
  (`GameplayStatics.PlaySoundAtLocation` "/Game/Sound/OFFer/Blend_Machine/OFFer_machine_Cue.OFFer_machine_Cue" (0.0 0.0 0.0) (struct) 1.0 1.0 0.0 null null null :!label _label))

(event `self.OFFer_spawn.OnComponentBeginOverlap`
  (params (OverlappedComponent :type "PrimitiveComponent Object Reference") (OtherActor :type "Actor Object Reference") (OtherComp :type "PrimitiveComponent Object Reference") (OtherBodyIndex :type Integer) (bFromSweep :type Boolean) (SweepResult :type "HitResult Structure (by ref)"))
  (bind _spawnlight (`self.SpawnLight`))
  (`SceneComponent.SetVisibility` _spawnlight (not (`SceneComponent.bVisible` _spawnlight)) false)
  (goto _label))

(event `self.Substance1.OnComponentBeginOverlap`
  (params (OverlappedComponent :type "PrimitiveComponent Object Reference") (OtherActor :type "Actor Object Reference") (OtherComp :type "PrimitiveComponent Object Reference") (OtherBodyIndex :type Integer) (bFromSweep :type Boolean) (SweepResult :type "HitResult Structure (by ref)"))
  ;[1 1 1] Substance
  (if (not (`self.DidSubstanceFill`))
    (`PrimitiveComponent.SetMaterial` (`self.Cube1`) 0 "/Game/Meshes/Blender_Machine/IsFiiled_Mat.IsFiiled_Mat")
    (cast `/Game/Meshes/Elements/BP_Fe` OtherActor
      (:`then`
        (set `self.Component1` "Fe"))
      (:`CastFailed`
        (cast `/Game/Meshes/Elements/BP_Zn` OtherActor
          (:`then`
            (set `self.Component1` "Zn"))
          (:`CastFailed`
            (cast `/Game/Meshes/Flaska/HCL/BP_FlaskaHCL` OtherActor
              (:`then`
                (set `self.Component1` "HCl"))
              (:`CastFailed`
                (cast `/Game/Meshes/Flaska/H2SO4/BP_FlaskaH2SO42` OtherActor
                  (:`then`
                    (set `self.Component1` "H2SO4"))
                  (:`CastFailed`
                    (cast `/Game/Meshes/Elements/BP_Mg` OtherActor
                      (:`then`
                        (set `self.Component1` "Mg"))
                      (:`CastFailed`
                        (cast `/Game/Meshes/Flaska/Secret/BP_FlaskaC6H4CH3_NO2_` OtherActor
                          (:`then`
                            (set `self.Component1` "S1"))
                          (:`CastFailed`
                            (cast `/Game/Meshes/Flaska/Secret/BP_FlaskaC6H3CH3_NO2_2` OtherActor)
                            (set `self.Component1` "S2")))))))))))))
    (set `self.DidSubstanceFill` true)))

(event `self.Substance1.OnComponentEndOverlap`
  (params (OverlappedComponent :type "PrimitiveComponent Object Reference") (OtherActor :type "Actor Object Reference") (OtherComp :type "PrimitiveComponent Object Reference") (OtherBodyIndex :type Integer))
  ;[1 1 1] Substance
  (set `self.Component1` "")
  (set `self.DidSubstanceFill` false)
  (`PrimitiveComponent.SetMaterial` (`self.Cube1`) 0 "/Game/Meshes/Blender_Machine/IsNotFiiled_Mat.IsNotFiiled_Mat"))

(event `self.Substance2.OnComponentBeginOverlap`
  (params (OverlappedComponent :type "PrimitiveComponent Object Reference") (OtherActor :type "Actor Object Reference") (OtherComp :type "PrimitiveComponent Object Reference") (OtherBodyIndex :type Integer) (bFromSweep :type Boolean) (SweepResult :type "HitResult Structure (by ref)"))
  ;[1 1 1] Substance 2
  (if (not (`self.DidSubstanceFill2`))
    (`PrimitiveComponent.SetMaterial` (`self.Cube2`) 0 "/Game/Meshes/Blender_Machine/IsFiiled_Mat.IsFiiled_Mat")
    (cast `/Game/Meshes/Elements/BP_Fe` OtherActor
      (:`then`
        (set `self.Component2` "Fe"))
      (:`CastFailed`
        (cast `/Game/Meshes/Elements/BP_Zn` OtherActor
          (:`then`
            (set `self.Component2` "Zn"))
          (:`CastFailed`
            (cast `/Game/Meshes/Flaska/HCL/BP_FlaskaHCL` OtherActor
              (:`then`
                (set `self.Component2` "HCl"))
              (:`CastFailed`
                (cast `/Game/Meshes/Flaska/H2SO4/BP_FlaskaH2SO42` OtherActor
                  (:`then`
                    (set `self.Component2` "H2SO4"))
                  (:`CastFailed`
                    (cast `/Game/Meshes/Elements/BP_Mg` OtherActor
                      (:`then`
                        (set `self.Component2` "Mg"))
                      (:`CastFailed`
                        (cast `/Game/Meshes/Flaska/Secret/BP_FlaskaC6H4CH3_NO2_` OtherActor
                          (:`then`
                            (set `self.Component2` "S1"))
                          (:`CastFailed`
                            (cast `/Game/Meshes/Flaska/Secret/BP_FlaskaC6H3CH3_NO2_2` OtherActor)
                            (set `self.Component2` "S2")))))))))))))
    (set `self.DidSubstanceFill2` true)))

(event `self.Substance2.OnComponentEndOverlap`
  (params (OverlappedComponent :type "PrimitiveComponent Object Reference") (OtherActor :type "Actor Object Reference") (OtherComp :type "PrimitiveComponent Object Reference") (OtherBodyIndex :type Integer))
  ;[1 1 1] Substance 2
  (set `self.Component2` "")
  (set `self.DidSubstanceFill2` false)
  (`PrimitiveComponent.SetMaterial` (`self.Cube2`) 0 "/Game/Meshes/Blender_Machine/IsNotFiiled_Mat.IsNotFiiled_Mat"))

(event `self.SoundTrigger.OnComponentBeginOverlap`
  (params (OverlappedComponent :type "PrimitiveComponent Object Reference") (OtherActor :type "Actor Object Reference") (OtherComp :type "PrimitiveComponent Object Reference") (OtherBodyIndex :type Integer) (bFromSweep :type Boolean) (SweepResult :type "HitResult Structure (by ref)"))
  ;[1 1 1] Fade in/out background sound of light
  (cast `/Game/VirtualRealityBP/Blueprints/BP_MotionController` OtherActor)
  (`AudioComponent.FadeIn` (`self.Audio`) 1.5 1.0 0.0 "Linear"))

(event `self.SoundTrigger.OnComponentEndOverlap`
  (params (OverlappedComponent :type "PrimitiveComponent Object Reference") (OtherActor :type "Actor Object Reference") (OtherComp :type "PrimitiveComponent Object Reference") (OtherBodyIndex :type Integer))
  ;[1 1 1] Fade in/out background sound of light
  (cast `/Game/VirtualRealityBP/Blueprints/BP_MotionController` OtherActor)
  (`AudioComponent.FadeOut` (`self.Audio`) 1.5 0.0 "Linear"))

(fn `Result`
  (bind _component1 (`self.Component1`))
  (bind _component1_2 (`self.Component1`))
  (bind _component2 (`self.Component2`))
  (bind _component1_3 (`self.Component1`))
  (bind _component2_2 (`self.Component2`))
  (bind _component1_4 (`self.Component1`))
  (bind _component2_3 (`self.Component2`))
  (bind _component2_4 (`self.Component2`))
  (bind _component1_5 (`self.Component1`))
  (bind _component2_5 (`self.Component2`))
  (bind _component1_6 (`self.Component1`))
  (bind _component2_6 (`self.Component2`))
  (bind _component1_7 (`self.Component1`))
  (bind _component2_7 (`self.Component2`))
  (bind (_returnvalue_location _returnvalue_rotation) (`KismetMathLibrary.BreakTransform` (`SceneComponent.K2_GetComponentToWorld` (`self.SpawnPoint`))))
  (bind (_returnvalue_location_2 _returnvalue_rotation_2) (`KismetMathLibrary.BreakTransform` (`SceneComponent.K2_GetComponentToWorld` (`self.SpawnPoint1`))))
  (bind (_returnvalue_location_3 _returnvalue_rotation_3) (`KismetMathLibrary.BreakTransform` (`SceneComponent.K2_GetComponentToWorld` (`self.SpawnPoint`))))
  (bind (_returnvalue_location_4 _returnvalue_rotation_4) (`KismetMathLibrary.BreakTransform` (`SceneComponent.K2_GetComponentToWorld` (`self.SpawnPoint`))))
  (bind (_returnvalue_location_5 _returnvalue_rotation_5) (`KismetMathLibrary.BreakTransform` (`SceneComponent.K2_GetComponentToWorld` (`self.SpawnPoint`))))
  (bind (_returnvalue_location_6 _returnvalue_rotation_6) (`KismetMathLibrary.BreakTransform` (`SceneComponent.K2_GetComponentToWorld` (`self.SpawnPoint`))))
  (bind (_returnvalue_location_7 _returnvalue_rotation_7) (`KismetMathLibrary.BreakTransform` (`SceneComponent.K2_GetComponentToWorld` (`self.SpawnPoint1`))))
  (if (not (and (`KismetStringLibrary.EqualEqual_StrStr` (`self.Component1`)) (`KismetStringLibrary.EqualEqual_StrStr` (`self.Component2`))))
    ;[1 1 1] FeCl2
    (if (or (and (`KismetStringLibrary.EqualEqual_StrStr` _component1_7 "Fe") (`KismetStringLibrary.EqualEqual_StrStr` _component2_4 "HCl")) (and (`KismetStringLibrary.EqualEqual_StrStr` _component1_7 "HCl") (`KismetStringLibrary.EqualEqual_StrStr` _component2_4 "Fe")))
      (`|SpawnActorFromClass` "/Game/Meshes/Flaska/FeCl2/BP_FlaskaFeCl2.BP_FlaskaFeCl2_C" (`KismetMathLibrary.MakeTransform` _returnvalue_location _returnvalue_rotation) "Undefined" "OverrideRootScale" null null)
      (`|SpawnActorFromClass` "/Game/Meshes/Flaska/H2/BP_FlaskaH2.BP_FlaskaH2_C" (`KismetMathLibrary.MakeTransform` _returnvalue_location_2 _returnvalue_rotation_2) "Undefined" "OverrideRootScale" null null :!label _label)
      (set `self.Component1` "" :!label _label_2)
      (set `self.Component2` "")
      (`GameplayStatics.PlaySoundAtLocation` "/Game/Sound/Noise/Smoke_Spawned/noise_of_smoke_spawned_1.noise_of_smoke_spawned_1" (`SceneComponent.K2_GetComponentLocation` (`self.SpawnPoint`)) (struct) 1.0 1.0 0.0 "/Game/Sound/Falling/Items_are_fell_Attenuation.Items_are_fell_Attenuation" null null)
      (`PrimitiveComponent.SetMaterial` (`self.Cube1`) 0 "/Game/Meshes/Blender_Machine/IsNotFiiled_Mat.IsNotFiiled_Mat")
      (`PrimitiveComponent.SetMaterial` (`self.Cube2`) 0 "/Game/Meshes/Blender_Machine/IsNotFiiled_Mat.IsNotFiiled_Mat")
      (else
        ;[1 1 1] ZnCL2
        (if (or (and (`KismetStringLibrary.EqualEqual_StrStr` _component1 "Zn") (`KismetStringLibrary.EqualEqual_StrStr` _component2_6 "HCl")) (and (`KismetStringLibrary.EqualEqual_StrStr` _component1 "HCl") (`KismetStringLibrary.EqualEqual_StrStr` _component2_6 "Zn")))
          (`|SpawnActorFromClass` "/Game/Meshes/Flaska/ZnCl2/BP_FlaskaZnCl2.BP_FlaskaZnCl2_C" (`KismetMathLibrary.MakeTransform` _returnvalue_location_3 _returnvalue_rotation_3) "Undefined" "OverrideRootScale" null null)
          (goto _label)
          (elif (or (and (`KismetStringLibrary.EqualEqual_StrStr` _component1_3 "Fe") (`KismetStringLibrary.EqualEqual_StrStr` _component2_2 "H2SO4")) (and (`KismetStringLibrary.EqualEqual_StrStr` _component1_3 "H2SO4") (`KismetStringLibrary.EqualEqual_StrStr` _component2_2 "Fe")))
            (`|SpawnActorFromClass` "/Game/Meshes/Flaska/FeSO4/BP_FlaskaFeSO4.BP_FlaskaFeSO4_C" (`KismetMathLibrary.MakeTransform` _returnvalue_location_4 _returnvalue_rotation_4) "Undefined" "OverrideRootScale" null null)
            (goto _label)
            (elif (or (and (`KismetStringLibrary.EqualEqual_StrStr` _component1_2 "Mg") (`KismetStringLibrary.EqualEqual_StrStr` _component2 "HCl")) (and (`KismetStringLibrary.EqualEqual_StrStr` _component1_2 "HCl") (`KismetStringLibrary.EqualEqual_StrStr` _component2 "Mg")))
              (`|SpawnActorFromClass` "/Game/Meshes/Flaska/MgCl2/BP_FlaskaMgCl2.BP_FlaskaMgCl2_C" (`KismetMathLibrary.MakeTransform` _returnvalue_location_5 _returnvalue_rotation_5) "Undefined" "OverrideRootScale" null null)
              (goto _label)
              (else
                ;[1 1 1] MgSO4
                (if (or (and (`KismetStringLibrary.EqualEqual_StrStr` _component1_4 "Mg") (`KismetStringLibrary.EqualEqual_StrStr` _component2_3 "H2SO4")) (and (`KismetStringLibrary.EqualEqual_StrStr` _component1_4 "H2SO4") (`KismetStringLibrary.EqualEqual_StrStr` _component2_3 "Mg")))
                  (`|SpawnActorFromClass` "/Game/Meshes/Flaska/MgSO4/BP_FlaskaMgSO4.BP_FlaskaMgSO4_C" (`KismetMathLibrary.MakeTransform` _returnvalue_location_6 _returnvalue_rotation_6 (1.0 1.0 1.0)) "Undefined" "OverrideRootScale" null null)
                  (goto _label)
                  (elif (or (and (`KismetStringLibrary.EqualEqual_StrStr` _component1_5 "H") (`KismetStringLibrary.EqualEqual_StrStr` _component2_5 "Cl")) (and (`KismetStringLibrary.EqualEqual_StrStr` _component1_5 "Cl") (`KismetStringLibrary.EqualEqual_StrStr` _component2_5 "H")))
                    (`|SpawnActorFromClass` "/Game/Meshes/Flaska/HCL/BP_FlaskaHCL.BP_FlaskaHCL_C" (`KismetMathLibrary.MakeTransform` _returnvalue_location_6 _returnvalue_rotation_6) "Undefined" "OverrideRootScale" null null)
                    (goto _label_2)
                    (elif (or (and (`KismetStringLibrary.EqualEqual_StrStr` _component1_6 "S1") (`KismetStringLibrary.EqualEqual_StrStr` _component2_7 "S2")) (and (`KismetStringLibrary.EqualEqual_StrStr` _component1_6 "S2") (`KismetStringLibrary.EqualEqual_StrStr` _component2_7 "S1")))
                      (`|SpawnActorFromClass` "/Game/Meshes/Flaska/DangerousFlaska/DBP_DangerousFlaska.DBP_DangerousFlaska_C" (`KismetMathLibrary.MakeTransform` _returnvalue_location_6 _returnvalue_rotation_6) "Undefined" "OverrideRootScale" null null)
                      (goto _label_2)
                      (elif (and (not (`KismetStringLibrary.IsEmpty` (`self.Component1`))) (not (`KismetStringLibrary.IsEmpty` (`self.Component2`))))
                        (`|SpawnActorFromClass` "/Game/Meshes/Flaska/DangerousFlaska/DBP_DangerousFlaska.DBP_DangerousFlaska_C" (`KismetMathLibrary.MakeTransform` _returnvalue_location_7 _returnvalue_rotation_7) "Undefined" "OverrideRootScale" null null)
                        (goto _label_2)))))))))))))

(fn `UserConstructionScript`)