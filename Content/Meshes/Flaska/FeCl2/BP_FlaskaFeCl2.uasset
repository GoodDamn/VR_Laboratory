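; BP_FlaskaFeCl2 is a FeCl2 flask actor that BP_MotionController can pick up.
; Pickup either breaks and clears a valid constraint or sets the constraint's components to join the hand and the flask's static mesh, then stores it.
; Drop is empty, and disconnected logic for releasing one of two constraints and promoting the second never runs.
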(event `/Game/VirtualRealityBP/Blueprints/PickupActorInterface.Pickup`
  (params (Constraint :type "PhysicsConstraintComponent Object Reference") (Hand :type "StaticMeshComponent Object Reference"))
  (bind _constraint (`self.Constraint`)
    (:`then`
      (`PhysicsConstraintComponent.BreakConstraint` _constraint)
      (set `self.Constraint` null))
    (:`else`
      (`PhysicsConstraintComponent.SetConstrainedComponents` Constraint Hand "None" (`self.StaticMeshComponent`) "None")
      (set `self.Constraint` Constraint))))

(event `/Game/VirtualRealityBP/Blueprints/PickupActorInterface.Drop`
  (params (Constraint :type "PhysicsConstraintComponent Object Reference")))

(fn `UserConstructionScript`)