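; BP_TheTray is a tray that motion controllers pick up and that makes a fall sound when it hits something.
; Pickup, called by BP_MotionController, either breaks a valid stored constraint or constrains the hand to the tray's static mesh, while Drop is empty.
; Component hits spawn an attenuated sound at the impact point, with volume mapped from velocity and a DoOnce reset after a short random delay to limit repeats.
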(event `/Game/VirtualRealityBP/Blueprints/PickupActorInterface.Pickup`
  (params (Constraint :type "PhysicsConstraintComponent Object Reference") (Hand :type "StaticMeshComponent Object Reference"))
  (bind _constraint (`self.Constraint`)
    (:`then`
      (`PhysicsConstraintComponent.BreakConstraint` _constraint)
      (set `self.Constraint` null))
    (:`else`
      (`PhysicsConstraintComponent.SetConstrainedComponents` Constraint Hand "None" (`self.StaticMeshComponent`) "None")
      (set `self.Constraint` Constraint))))

(event `/Game/VirtualRealityBP/Blueprints/PickupActorInterface.Drop`
  (params (Constraint :type "PhysicsConstraintComponent Object Reference")))

(event `self.StaticMeshComponent.OnComponentHit`
  (params (HitComponent :type "PrimitiveComponent Object Reference") (OtherActor :type "Actor Object Reference") (OtherComp :type "PrimitiveComponent Object Reference") (NormalImpulse :type "Vector Structure") (Hit :type "HitResult Structure (by ref)"))
  (`|ExecutionSequence`
    (:`then_0`
      (`/Engine/EditorBlueprintResources/StandardMacros.DoOnce` true :!label _label
        (:`Completed`
          (bind _returnvalue (`GameplayStatics.SpawnSoundAtLocation` "/Game/Sound/Falling/Sound_of_fallen_tray_Cue.Sound_of_fallen_tray_Cue" (`.Location` (`GameplayStatics.BreakHitResult` Hit)) (struct) 1.0 1.0 0.0 "/Game/Sound/Falling/Items_are_fell_Attenuation.Items_are_fell_Attenuation" null))
          (set `AudioComponent.VolumeMultiplier` (`KismetMathLibrary.MapRangeClamped` (`KismetMathLibrary.VSize` (`self.GetVelocity`)) 30.0 0.0 1.0) _returnvalue))))
    (:`then_1`
      (`KismetSystemLibrary.Delay` (`KismetMathLibrary.RandomFloatInRange` 0.1 0.2))
      (goto _label :!via `Reset`))))

(fn `UserConstructionScript`)