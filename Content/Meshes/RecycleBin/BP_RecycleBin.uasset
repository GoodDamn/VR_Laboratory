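; VR recycle bin that can be picked up and destroys objects that enter its Delete volume, playing a rubbish sound.
; Pickup, called by BP_MotionController, constrains the mesh to the hand, with two constraint slots tracked so Drop releases the matching one.
; A chain of failed casts on overlap exempts controllers, trigger boxes and specific lab and menu actors from deletion.
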(event `/Game/VirtualRealityBP/Blueprints/PickupActorInterface.Pickup`
  (params (Constraint :type "PhysicsConstraintComponent Object Reference") (Hand :type "StaticMeshComponent Object Reference"))
  (`PhysicsConstraintComponent.SetConstrainedComponents` Constraint Hand "None" (`self.StaticMeshComponent`) "None")
  (`self.Constraint`
    (:`then`
      (set `self.Constraint2` Constraint))
    (:`else`
      (set `self.Constraint` Constraint))))

(event `/Game/VirtualRealityBP/Blueprints/PickupActorInterface.Drop`
  (params (Constraint :type "PhysicsConstraintComponent Object Reference"))
  (bind _constraint (`self.Constraint`)
    (:`then`
      (if (== _constraint Constraint)
        (`PhysicsConstraintComponent.BreakConstraint` (`self.Constraint`))
        (set `self.Constraint` null)
        (bind _constraint2 (`self.Constraint2`)
          (:`then`
            (set `self.Constraint` _constraint2)
            (set `self.Constraint2` null))
          (:`else`))
        (else
          (bind _constraint2_2 (`self.Constraint2`)
            (:`then`
              (if (== _constraint2_2 Constraint)
                (`PhysicsConstraintComponent.BreakConstraint` (`self.Constraint2`))
                (set `self.Constraint2` null)))
            (:`else`)))))
    (:`else`)))

(event `self.Delete.OnComponentBeginOverlap`
  (params (OverlappedComponent :type "PrimitiveComponent Object Reference") (OtherActor :type "Actor Object Reference") (OtherComp :type "PrimitiveComponent Object Reference") (OtherBodyIndex :type Integer) (bFromSweep :type Boolean) (SweepResult :type "HitResult Structure (by ref)"))
  (cast `/Game/VirtualRealityBP/Blueprints/BP_MotionController` OtherActor
    (:`CastFailed`
      (cast `/Game/Widgets/Widgets/Interactive/Theory_IBP` OtherActor
        (:`CastFailed`
          (cast `/Game/Widgets/Widgets/Interactive/Quit_BP` OtherActor
            (:`CastFailed`
              (cast `/Game/Widgets/Widgets/Interactive/Practice_IBP` OtherActor
                (:`CastFailed`
                  (cast `/Game/Meshes/Blender_Machine/BP_blend_machine` OtherActor
                    (:`CastFailed`
                      (cast `TriggerBox` OtherActor
                        (:`CastFailed`
                          (cast `/Game/Widgets/Widgets/Interactive/BP_Mendeleevs_table` OtherActor
                            (:`CastFailed`
                              (cast `/Game/Meshes/Washbasin/BP_Washbasin` OtherActor
                                (:`CastFailed`
                                  (cast `/Game/Meshes/Shelf/BP_shelf` OtherActor
                                    (:`CastFailed`
                                      (`self.K2_DestroyActor` OtherActor)
                                      (`GameplayStatics.PlaySound2D` "/Game/Sound/Rubbish/rubbish.rubbish" 1.0 1.0 0.0 null null))))))))))))))))))))

(fn `UserConstructionScript`)